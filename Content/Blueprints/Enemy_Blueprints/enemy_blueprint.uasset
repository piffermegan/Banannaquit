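; Enemy actor that flies along the world Y axis while bobbing up and down in a sine wave, apparently a bird.
; BeginPlay stores the start location, and Tick sets an absolute, unswept position from it using accumulated time, EnemySpeed, SineMult and BirdHeight.
; The overlap event is empty, and a backup forward-movement node is left unconnected.
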(event `self.ReceiveBeginPlay`
  (set `self.start_location` (`self.K2_GetActorLocation`)))

(event `self.ReceiveTick`
  (params (DeltaSeconds :type "Float (single-precision)"))
  (set `self.Total_Time` (+ DeltaSeconds (`self.Total_Time`)))
  (`self.K2_SetActorLocation` (+ (`KismetMathLibrary.MakeVector` 0.0 (* (`self.Enemy_Speed`) (`self.Total_Time`)) (* (`KismetMathLibrary.DegSin` (* (`self.Total_Time`) (`self.Sine_Mult`))) (`self.Bird_Height`))) (`self.start_location`))))

(fn `UserConstructionScript`)